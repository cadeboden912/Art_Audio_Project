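; AI character Blueprint that shows its health on a widget nameplate.
; On BeginPlay it runs the parent logic, waits briefly, then sets the nameplate progress bar's health range and current value through interface messages.
; Its health modify override calls the parent, then pushes the updated current health to the same bar.
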(event EventBeginPlay
  (bind _widget_nameplate (Variables|Default|GetWidget_Nameplate))
  (bind _returnvalue (UserInterface|GetUserWidgetObject _widget_nameplate))
  (bind _asw_nameplate (Utilities|Casting|CastToW_Nameplate _returnvalue))
  (bind _progressbar_health (Variables|/Game/Coursera/Widgets/HUD/W_Nameplate/W_Nameplate.W_Nameplate_C|GetProgressBar_Health _asw_nameplate))
  (|CallParentFunction)
  (Utilities|FlowControl|Delay 0.2)
  (Class|ProgressBarTemplete|InterfaceProgressBarSetMinMax(Message) _progressbar_health (Variables|Default|GetHealth_Minimum) (Variables|Default|GetHealth_Maximum))
  (Class|ProgressBarTemplete|InterfaceProgressBarUpdateCurrent(Message) _progressbar_health (Variables|Default|GetHealth_Current)))

(event Collision|EventActorBeginOverlap
  (params (OtherActor :type Actor%20Object%20Reference)))

(event EventTick
  (params (DeltaSeconds :type Float%20%28single-precision%29)))

(fn ConstructionScript
  (|CallParentFunction))

(fn FhealthModify
  (|CallParentFunction)
  (Class|ProgressBarTemplete|InterfaceProgressBarUpdateCurrent(Message) (Variables|/Game/Coursera/Widgets/HUD/W_Nameplate/W_Nameplate.W_Nameplate_C|GetProgressBar_Health (.AsW%20Nameplate (Utilities|Casting|CastToW_Nameplate (UserInterface|GetUserWidgetObject (Variables|Default|GetWidget_Nameplate))))) (Variables|Default|GetHealth_Current)))