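; BP_AI_Shield is a melee AI character, apparently the shield variant, built on a parent AI class that it extends with a sword attack.
; Its attack event calls the parent, plays a sped-up sword slash montage and passes notify begins to melee collision with fixed weapon damage.
; It supplies its weapon hitbox through a getter; overlaps on that hitbox apply damage to actors that pass the character-type interface check.
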(event OnComponentBeginOverlap(Weapon_Hitbox)
  (params (OverlappedComponent :type Primitive%20Component%20Object%20Reference) (OtherActor :type Actor%20Object%20Reference) (OtherComp :type Primitive%20Component%20Object%20Reference) (OtherBodyIndex :type Integer) (bFromSweep :type Boolean) (SweepResult :type Hit%20Result%20Structure%20%28by%20ref%29))
  (bind _player (Class|InterfaceCharatcerMaster|InterfaceCharacterType(Message) OtherActor))
  (if _player
    (CallFunction|FDamageApply OtherActor)))

(event EventBeginPlay
  (|CallParentFunction) ; This node is disabled and will not be called.\nDrag off pins to build functionality.
)

(event Collision|EventActorBeginOverlap
  (params (OtherActor :type Actor%20Object%20Reference)))

(event EventTick
  (params (DeltaSeconds :type Float%20%28single-precision%29)))

(event EventFAIAttack
  ;[0.15 0.15 0.15 0.5] Converted to Event
  ;[0.15 0.15 0.15 0.5] Upon range play attack animation
  (|CallParentFunction)
  (bind _notifyname (Animation|Montage|PlayMontage (Variables|Character|GetMesh) "/Game/Coursera/Mixemo/Animations/Attacks/Sword_shield/Sword_Slash_Montage.Sword_Slash_Montage" 1.5 0.0 "None" false)
    (:OnNotifyBegin
      (CallFunction|FMeleeCollision 2e+01 _notifyname true))))

(fn ConstructionScript
  (|CallParentFunction))

(fn FGetMeleeHitbox
  (params (Weapon :type Boolean))
  (return (Variables|Default|GetWeapon_Hitbox)))