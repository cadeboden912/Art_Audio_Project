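; BP_AI_Rifle is a rifle-wielding AI character that extends a parent AI Blueprint with a ranged attack.
; FAIAttack calls the parent logic, then plays the rifle montage on the mesh at increased speed.
; The montage's Notify Begin calls FSpawnProjectile at the gun's Muzzle socket, passing the notify name, so shots follow the animation's timing.
; The other events and construction script add no logic of their own.
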(event EventBeginPlay
  (|CallParentFunction) ; This node is disabled and will not be called.\nDrag off pins to build functionality.
)

(event Collision|EventActorBeginOverlap
  (params (OtherActor :type Actor%20Object%20Reference))
  (|CallParentFunction OtherActor))

(event EventTick
  (params (DeltaSeconds :type Float%20%28single-precision%29))
  (|CallParentFunction DeltaSeconds))

(event EventFAIAttack
  (|CallParentFunction)
  (bind _notifyname (Animation|Montage|PlayMontage (Variables|Character|GetMesh) "/Game/Coursera/Mixemo/Animations/Attacks/Rifle/Rifle_Montage.Rifle_Montage" 3.0)
    (:OnNotifyBegin
      (CallFunction|FSpawnProjectile (Variables|Default|GetGun) "Muzzle" 0.0 5e+01 2e+03 _notifyname "0.300000,0.300000,0.300000" 0.0 false "0, 0, 0" false))))

(fn ConstructionScript
  (|CallParentFunction))