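; BP_AI_Bow is an AI character Blueprint for a bow-wielding attacker that fires projectiles.
; It extends a parent class, calling the parent's FAIAttack before playing the bow montage on its mesh.
; When a montage notify begins, FSpawnProjectile launches a stretched projectile from the Bow mesh's arrow socket, so the shot follows the animation's timing.
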(event EventBeginPlay
  (|CallParentFunction) ; This node is disabled and will not be called.\nDrag off pins to build functionality.
)

(event Collision|EventActorBeginOverlap
  (params (OtherActor :type Actor%20Object%20Reference))
  (|CallParentFunction OtherActor))

(event EventTick
  (params (DeltaSeconds :type Float%20%28single-precision%29))
  (|CallParentFunction DeltaSeconds))

(event EventFAIAttack
  (|CallParentFunction)
  (bind _notifyname (Animation|Montage|PlayMontage (Variables|Character|GetMesh) "/Game/Coursera/Mixemo/Animations/Attacks/Bow/Bow_Montage.Bow_Montage")
    (:OnNotifyBegin
      (CallFunction|FSpawnProjectile (Variables|Default|GetBow) "S_Arrow" 0.0 5e+01 3e+03 _notifyname "2.000000,0.300000,0.300000" 0.0 false "0, 0, 0" false))))

(fn ConstructionScript
  (|CallParentFunction))