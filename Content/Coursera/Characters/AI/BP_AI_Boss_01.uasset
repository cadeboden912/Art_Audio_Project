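; Boss AI character with a great sword, built on a parent AI class that supplies the attack event.
; Each attack randomly plays a jump, casting or kick montage, whose notifies call the melee collision function with damage and weapon flag.
; Weapon hitbox overlaps apply damage to actors passing the character-type interface check, and an override exposes that hitbox.
; An alternative fixed attack rotation using AttackIndex is present but unconnected.
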(event OnComponentBeginOverlap(Weapon_Hitbox)
  (params (OverlappedComponent :type Primitive%20Component%20Object%20Reference) (OtherActor :type Actor%20Object%20Reference) (OtherComp :type Primitive%20Component%20Object%20Reference) (OtherBodyIndex :type Integer) (bFromSweep :type Boolean) (SweepResult :type Hit%20Result%20Structure%20%28by%20ref%29))
  (bind _player (Class|InterfaceCharatcerMaster|InterfaceCharacterType(Message) OtherActor))
  (if _player
    (CallFunction|FDamageApply OtherActor)))

(event EventBeginPlay
  (|CallParentFunction) ; This node is disabled and will not be called.\nDrag off pins to build functionality.
)

(event Collision|EventActorBeginOverlap
  (params (OtherActor :type Actor%20Object%20Reference)))

(event EventTick
  (params (DeltaSeconds :type Float%20%28single-precision%29)))

(event EventFAIAttack
  ;[0.15 0.15 0.15 0.5] Connect to whichever i want NPC attacks to go through
  (|CallParentFunction)
  ;[0.15 0.15 0.15 0.5] RNG (Random Number Generator) Version Random of the chosen attacks will be played
  (switch int (Math|Random|RandomIntegerinRange 1 3)
    (:1
      (bind _notifyname (Animation|Montage|PlayMontage (Variables|Character|GetMesh) "/Game/Coursera/Mixemo/Animations/Attacks/Two_Handed/GreatSwordJumpAttack_Montage.GreatSwordJumpAttack_Montage" 1.5 0.0 "None" false)
        (:OnNotifyBegin
          (CallFunction|FMeleeCollision 2e+01 _notifyname true))))
    (:2
      (bind _notifyname_2 (Animation|Montage|PlayMontage (Variables|Character|GetMesh) "/Game/Coursera/Mixemo/Animations/Attacks/Two_Handed/Great_Sword_Casting_02_Montage.Great_Sword_Casting_02_Montage")
        (:OnNotifyBegin
          (CallFunction|FMeleeCollision 2e+01 _notifyname_2 true))))
    (:3
      (bind _notifyname_3 (Animation|Montage|PlayMontage (Variables|Character|GetMesh) "/Game/Coursera/Mixemo/Animations/Attacks/Two_Handed/Great_Sword_Kick_Montage.Great_Sword_Kick_Montage")
        (:OnNotifyBegin
          (CallFunction|FMeleeCollision 2e+01 _notifyname_3 true))))))

(fn ConstructionScript
  (|CallParentFunction))

(fn FGetMeleeHitbox
  (params (Weapon :type Boolean))
  (return (Variables|Default|GetWeapon_Hitbox)))