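; Master AI character for enemies that patrol, detect and chase the player, with a nameplate health bar and optional jump-on damage.
; Patrols ping-pong along tag-ordered markers; accumulated detection escalates from looking to investigating to aggro, also triggered by sphere overlap or damage.
; Looping timers drive range-checked attacks, where the base attack only faces the target.
; Leash distance or target death resets health and target, optionally returning it to spawn or route.
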(event OnComponentBeginOverlap(Jump_hit)
  (params (OverlappedComponent :type Primitive%20Component%20Object%20Reference) (OtherActor :type Actor%20Object%20Reference) (OtherComp :type Primitive%20Component%20Object%20Reference) (OtherBodyIndex :type Integer) (bFromSweep :type Boolean) (SweepResult :type Hit%20Result%20Structure%20%28by%20ref%29))
  (bind _ascharacter (Utilities|Casting|CastToCharacter OtherActor))
  (bind _charactermovement (Variables|/Script/Engine.Character|GetCharacterMovement _ascharacter))
  ;[0.15 0.15 0.15 0.5] Reaction to jumped on by player
  (if (AI|Components|NavMovement|IsFalling _charactermovement)
    (if (> (.z (Transformation|GetActorLocation OtherActor)) (.z (Transformation|GetActorLocation)))
      (if (< (.z (Variables|/Script/Engine.MovementComponent|GetVelocity _charactermovement)) 0.0)
        ;;[0.15 0.15 0.15 0.5] Collide With Platform Collision
        (Class|AbilityActivateInterface|InterfaceJumpHitMontage(Message) OtherActor)
        (Class|InterfaceCharatcerMaster|InterfaceHealthModify(Message) self 5.0 "NewEnumerator1")
        (Animation|Montage|PlayMontage (Variables|Character|GetMesh) "/Game/Coursera/Mixemo/Animations/IsHIt/AS_Hit_Behind_Montage.AS_Hit_Behind_Montage")))))

(event OnComponentBeginOverlap(CollisionSphereaggro)
  (params (OverlappedComponent :type Primitive%20Component%20Object%20Reference) (OtherActor :type Actor%20Object%20Reference) (OtherComp :type Primitive%20Component%20Object%20Reference) (OtherBodyIndex :type Integer) (bFromSweep :type Boolean) (SweepResult :type Hit%20Result%20Structure%20%28by%20ref%29))
  ;[0.15 0.15 0.15 0.5] Approuch Character
  (bind _player (Class|InterfaceCharatcerMaster|InterfaceCharacterType(Message) OtherActor))
  (if _player
    (Movement|FAggroPlayer OtherActor)))

(event Custom|ceSpawnLocation_Leash
  ;[0.15 0.15 0.15 0.5] Distance where NPC can see player
  (if (not (Utilities|Time|IsTimerActivebyHandle (Variables|Spawn|GetTimer_Leash_Distance)))
    (bind _returnvalue (Utilities|Time|SetTimerbyEvent (delegate Custom|ceCheck_Leash_Distance) 2.0))
    (Variables|Spawn|SetTimer_Leash_Distance _returnvalue)))

(event Custom|ceCheck_Leash_Distance
  ;[0.15 0.15 0.15 0.5] Distance where NPC can see player
  (if (> (Utilities|Array|Length (Variables|Patrol|GetPatrol_Route)) 0)
    (if (> (Math|Vector|Distance(Vector) (Transformation|GetActorLocation) (Variables|Patrol|GetPatrol_Destination_old)) (Variables|Spawn|GetLeash%20Distance))
      (Components|Movement|StopMovementImmediately (Variables|Character|GetCharacterMovement) :!label _label)
      (Collision|SetCollisionEnabled (Variables|Default|GetCollision%20Sphere%20aggro) "NoCollision")
      ;[0.15 0.15 0.15 0.5] Reeset AI
      ;;[0.15 0.15 0.15 0.5] Reset AI Health
      (Variables|Default|SetHealth_Current (Variables|Default|GetHealth_Maximum))
      (Variables|Default|SetReset true)
      (Variables|Default|SetTarget 0)
      (Utilities|Time|ClearandInvalidateTimerbyHandle (Variables|Combat|GetTimer_Attack_Rotation))
      ;;[0.15 0.15 0.15 0.5] Send AI back to spawn
      (if (Variables|Default|GetGoes%20back%20to%20route)
        (bind _returnvalue (Utilities|Time|SetTimerbyEvent (delegate Custom|ceCheckforSpawnLocation) 1.0 true))
        (Variables|Spawn|SetTimer_CheckforSpawnLocation _returnvalue)
        ;[0.15 0.15 0.15 0.5] Reset Spot in route
        (if (> (Utilities|Array|Length (Variables|Patrol|GetPatrol_Route)) 0)
          (Movement|FAIMoveto false (Variables|Patrol|GetPatrol_Destination_old))
          (else
            (Movement|FAIMoveto false (Variables|Spawn|GetSpawn_Location))))))
    (elif (> (Math|Vector|Distance(Vector) (Transformation|GetActorLocation) (Variables|Spawn|GetSpawn_Location)) (Variables|Spawn|GetLeash%20Distance))
      (goto _label))))

(event Custom|ceReset_AI_Character
  ;[0.15 0.15 0.15 0.5] Distance where NPC can see player
  (Components|Movement|StopMovementImmediately (Variables|Character|GetCharacterMovement))
  (Collision|SetCollisionEnabled (Variables|Default|GetCollision%20Sphere%20aggro) "NoCollision")
  ;[0.15 0.15 0.15 0.5] Reeset AI
  ;;[0.15 0.15 0.15 0.5] Reset AI Health
  (Variables|Default|SetHealth_Current (Variables|Default|GetHealth_Maximum))
  (Variables|Default|SetReset true)
  (Variables|Default|SetTarget 0)
  (Utilities|Time|ClearandInvalidateTimerbyHandle (Variables|Combat|GetTimer_Attack_Rotation))
  ;;[0.15 0.15 0.15 0.5] Send AI back to spawn
  (if (Variables|Default|GetGoes%20back%20to%20route)
    (bind _returnvalue (Utilities|Time|SetTimerbyEvent (delegate Custom|ceCheckforSpawnLocation) 1.0 true))
    (Variables|Spawn|SetTimer_CheckforSpawnLocation _returnvalue)
    ;[0.15 0.15 0.15 0.5] Reset Spot in route
    (if (> (Utilities|Array|Length (Variables|Patrol|GetPatrol_Route)) 0)
      (Movement|FAIMoveto false (Variables|Patrol|GetPatrol_Destination_old))
      (else
        (Movement|FAIMoveto false (Variables|Spawn|GetSpawn_Location))))))

(event Custom|ceCheckforSpawnLocation
  ;[0.15 0.15 0.15 0.5] Reeset AI
  ;;[0.15 0.15 0.15 0.5] Send AI back to spawn
  (if (> (Utilities|Array|Length (Variables|Patrol|GetPatrol_Route)) 0)
    (if (> (Math|Vector|Distance(Vector) (Transformation|GetActorLocation) (Variables|Patrol|GetPatrol_Destination_old)) 5e+01)
      (Utilities|Time|ClearandInvalidateTimerbyHandle (Variables|Spawn|GetTimer_Leash_Distance) :!label _label)
      ;;[0.15 0.15 0.15 0.5] Reenable Collision
      (Collision|SetCollisionEnabled (Variables|Default|GetCollision%20Sphere%20aggro) "QueryOnly")
      ;;[0.15 0.15 0.15 0.5] Final Reset
      (Utilities|Time|ClearandInvalidateTimerbyHandle (Variables|Spawn|GetTimer_CheckforSpawnLocation))
      ;;[0.15 0.15 0.15 0.5] Back to undetected
      (Variables|Detection|SetPlayer_Detection 0)
      (Variables|Default|SetReset false)
      (if (> (Utilities|Array|Length (Variables|Patrol|GetPatrol_Route)) 0)
        (CallFunction|CePatrolRoute)))
    (elif (> (Math|Vector|Distance(Vector) (Transformation|GetActorLocation) (Variables|Spawn|GetSpawn_Location)) 5e+01)
      (goto _label))))

(event Custom|ceTrigger_Attack
  ;[0.15 0.15 0.15 0.5] Every time AI attacks
  (bind _returnvalue (Utilities|Time|SetTimerbyEvent (delegate Custom|ceAttack_Range) 0.25 true))
  (Variables|Combat|SetTimer_Attack_Rotation _returnvalue))

(event Custom|ceAttack_Range
  (Utilities|IsValid (Variables|Default|GetTarget)
    (:Is%20Valid
      (if (not (Variables|Default|GetDead))
        (if (not (Variables|Default|GetReset))
          (bind _dead (Class|InterfaceCharatcerMaster|InterfaceGetDeadState(Message) (Variables|Default|GetTarget)))
          (if _dead
            (CallFunction|CeResetAICharacter)
            (elif (<= (Math|Vector|Distance(Vector) (Transformation|GetActorLocation (Variables|Default|GetTarget)) (Transformation|GetActorLocation)) (Variables|Combat|GetAttack%20Range))
              (Utilities|FlowControl|DoOnce false
                (:Completed
                  (CallFunction|FAIAttack)
                  (Utilities|FlowControl|Delay (Variables|Combat|GetAttack%20speed))
                  (CallFunction|CeAttackReset)))
              (else
                (Movement|FAIMoveto true "0, 0, 0" (Variables|Default|GetTarget))))))))))

(event Custom|ceAttack_Reset
  (Utilities|FlowControl|DoOnce false) ; enters at Reset
)

(event Custom|cePatrol_Route
  (bind _patrol_route (Variables|Patrol|GetPatrol_Route))
  (bind _patrol_index (Variables|Patrol|GetPatrol_Index))
  (bind _output (Utilities|Array|Get(acopy) _patrol_route _patrol_index))
  (bind _returnvalue (Transformation|GetActorLocation _output))
  (if (> (Utilities|Array|Length (Variables|Patrol|GetPatrol_Route)) 0)
    (if (not (Variables|Default|GetDead))
      (CallFunction|FmovespeedWalk)
      (Movement|FAIMoveto false _returnvalue)
      (Variables|Patrol|SetPatrol_Destination _returnvalue)
      (bind _returnvalue_2 (Utilities|Time|SetTimerbyEvent (delegate Custom|ceCheck_Patrol_Destination) 1.0 true))
      (Variables|Patrol|SetTimer_Patrol_Route _returnvalue_2))))

(event Custom|ceCheck_Patrol_Destination
  (if (<= (Math|Vector|Distance(Vector) (Transformation|GetActorLocation) (Variables|Patrol|GetPatrol_Destination)) 1.5e+02)
    (if (Variables|Patrol|GetPatrol_Reverse)
      ;[0.15 0.15 0.15 0.5] Reverse of below
      (bind _result (Math|Integer|DecrementInt (Variables|Patrol|GetPatrol_Index))
        (:%20%20
          (if (== _result 0)
            (Variables|Patrol|SetPatrol_Reverse false)
            (Variables|Patrol|SetPatrol_Index 1))))
      (else
        ;[0.15 0.15 0.15 0.5] If patrol route is trying to be greater then the last of the listed index, it will reverse
        (bind _result_2 (Math|Integer|IncrementInt (Variables|Patrol|GetPatrol_Index))
          (:%20%20
            (if (> _result_2 (Utilities|Array|LastIndex (Variables|Patrol|GetPatrol_Route)))
              (Variables|Patrol|SetPatrol_Reverse true)
              (Variables|Patrol|SetPatrol_Index (- (Utilities|Array|LastIndex (Variables|Patrol|GetPatrol_Route)) 1)))))))
    (Utilities|Time|ClearandInvalidateTimerbyHandle (Variables|Patrol|GetTimer_Patrol_Route))
    (Utilities|FlowControl|Delay (Math|Random|RandomFloatinRange 1.0 3.0))
    (CallFunction|CePatrolRoute)
    (Variables|Patrol|SetPatrol_Destination_old (Variables|Patrol|GetPatrol_Destination))))

(event Custom|ceReset_Patrol
  ;[0.15 0.15 0.15 0.5] AI to player movement
  (CallFunction|CePatrolRoute))

(event EventBeginPlay
  (bind _widget_nameplate (Variables|Default|GetWidget_Nameplate))
  (bind _returnvalue (UserInterface|GetUserWidgetObject _widget_nameplate))
  (bind _asw_nameplate (Utilities|Casting|CastToW_Nameplate _returnvalue))
  (bind _progressbar_health (Variables|/Game/Coursera/Widgets/HUD/W_Nameplate/W_Nameplate.W_Nameplate_C|GetProgressBar_Health _asw_nameplate))
  ;[0.15 0.15 0.15 0.5] AI_Healthbar
  (|CallParentFunction)
  (Utilities|FlowControl|Delay 2.0)
  (CallFunction|FAISetAnimationStance)
  (Class|ProgressBarTemplete|InterfaceProgressBarSetMinMax(Message) _progressbar_health (Variables|Default|GetHealth_Minimum) (Variables|Default|GetHealth_Maximum))
  (Class|ProgressBarTemplete|InterfaceProgressBarUpdateCurrent(Message) _progressbar_health (Variables|Default|GetHealth_Current))
  ;[0.15 0.15 0.15 0.5] Set AI spawn Location
  (Variables|Spawn|SetSpawn_Location (Transformation|GetActorLocation))
  ;[0.15 0.15 0.15 0.5] Is Platformer Type
  (if (Variables|Combat|GetIsPlatfomer)
    (Collision|SetCollisionEnabled (Variables|Default|GetJump_hit) "QueryOnly")))

(event EventInterfaceDetectPlayer
  (params (Actor :type Actor%20Object%20Reference) (Value :type Integer))
  ;[0.15 0.15 0.15 0.5] AI to player movement
  ;;[0.15 0.15 0.15 0.5] Reset all noise upon reset
  (if (not (Variables|Default|GetReset))
    (Variables|Detection|SetPlayer_Detected Actor)
    (bind _output_get (Variables|Detection|SetPlayer_Detection (+ Value (Variables|Detection|GetPlayer_Detection))))
    (if (not (<= (Variables|Detection|GetPlayer_Detection) 33))
      (if (<= _output_get 50)
        ;;[0.15 0.15 0.15 0.5] Look at Player
        (Transformation|SetActorRotation (Math|Rotator|FindLookatRotation (Transformation|GetActorLocation) (Transformation|GetActorLocation (Variables|Detection|GetPlayer_Detected))))
        ;;[0.15 0.15 0.15 0.5] Stops Noise and Route interfierance
        (Utilities|Time|ClearandInvalidateTimerbyHandle (Variables|Patrol|GetTimer_Patrol_Route))
        (Components|Movement|StopMovementImmediately (Variables|Character|GetCharacterMovement))
        (bind _returnvalue (Utilities|Time|SetTimerbyEvent (delegate Custom|ceReset_Patrol) 1e+01 :!label _label))
        (Variables|Patrol|SetReset_Patrol _returnvalue)
        (elif (<= (Variables|Detection|GetPlayer_Detection) 80)
          ;;[0.15 0.15 0.15 0.5] Walk to player location
          ;;;[0.15 0.15 0.15 0.5] Stops Noise and Route interfierance
          (Utilities|Time|ClearandInvalidateTimerbyHandle (Variables|Patrol|GetTimer_Patrol_Route))
          (Components|Movement|StopMovementImmediately (Variables|Character|GetCharacterMovement))
          (CallFunction|FmovespeedWalk)
          (Movement|FAIMoveto false (Transformation|GetActorLocation (Variables|Detection|GetPlayer_Detected)))
          (CallFunction|CeSpawnLocationLeash)
          (goto _label)
          (elif (>= (Variables|Detection|GetPlayer_Detection) 100)
            ;;[0.15 0.15 0.15 0.5] Attack Player
            (Movement|FAggroPlayer (Variables|Detection|GetPlayer_Detected))))))))

(event EventInterfaceSetAIOwner
  (params (Owner :type Actor%20Object%20Reference))
  ;[0.15 0.15 0.15 0.5] Set AI as the owner
  (Actor|SetOwner Owner))

(event EventInterfaceSetAIPatrolRoute
  (params (Patrol%20Route :type Name :default "None"))
  (if (not (== Patrol%20Route ""))
    ;[0.15 0.15 0.15 0.5] Retrieve all Patrol Actors
    (bind _outactors (Actor|GetAllActorsOfClasswithTag "/Game/Coursera/Actors/Actor_Patrol_Marker/Actor_Patrol_Marker.Actor_Patrol_Marker_C" Patrol%20Route))
    (for _array_element _outactors
      ;[0.15 0.15 0.15 0.5] Gets from listed tags to define the route
      (Utilities|Array|SetArrayElem (Variables|Patrol|GetPatrol_Route) (Math|Conversions|ToInteger(Byte) (Utilities|String|ToString(Name) (Utilities|Array|Get(acopy) (Variables|/Script/Engine.Actor|GetTags _array_element)))) _array_element true))
    ;[0.15 0.15 0.15 0.5] After each destination make AI have a short delay
    (Utilities|FlowControl|Delay (Math|Random|RandomFloatinRange 1.0 2.0))
    (CallFunction|CePatrolRoute)))

(fn ConstructionScript
  (|CallParentFunction)
  (if (Variables|Detection|GetPlayer_Detection_System_Only)
    (Variables|/Script/Engine.PrimitiveComponent|SetbGenerateOverlapEvents (Variables|Default|GetCollision%20Sphere%20aggro) false)))

(fn FhealthModify
  (|CallParentFunction)
  (Class|ProgressBarTemplete|InterfaceProgressBarUpdateCurrent(Message) (Variables|/Game/Coursera/Widgets/HUD/W_Nameplate/W_Nameplate.W_Nameplate_C|GetProgressBar_Health (.AsW%20Nameplate (Utilities|Casting|CastToW_Nameplate (UserInterface|GetUserWidgetObject (Variables|Default|GetWidget_Nameplate))))) (Variables|Default|GetHealth_Current)))

(fn FDead
  (|CallParentFunction)
  (Class|InterfaceSpawnerAI|Respawn(Message) (Components|GetOwner))
  (Utilities|Time|SetTimerbyEvent (EventDispatchers|CreateEvent :!event K2DestroyActor) 2.0)
  (Components|Movement|StopMovementImmediately (Variables|Character|GetCharacterMovement)))

(fn InterfaceCharacterType
  (return false))

(fn FAggroPlayer
  (params (Player :type Actor%20Object%20Reference))
  (Movement|FAIMoveto true "0, 0, 0" Player)
  (CallFunction|CeSpawnLocationLeash)
  (CallFunction|F:movespeedRun)
  (Variables|Default|SetTarget Player)
  (Development|PrintString (Utilities|GetDisplayName Player) true true "(R=0.000000,G=0.660000,B=1.000000,A=1.000000)" 1e+01)
  (CallFunction|CeTriggerAttack)
  (Utilities|Time|ClearandInvalidateTimerbyHandle (Variables|Patrol|GetTimer_Patrol_Route))
  (Utilities|Time|ClearandInvalidateTimerbyHandle (Variables|Patrol|GetReset_Patrol)))

(fn FAIMoveto
  (params (Use%20Actor :type Boolean) (Location :type Vector) (Actor :type Actor%20Object%20Reference))
  (if (not (Variables|Default|GetDead))
    (if Use%20Actor
      (if (not (Variables|Default|GetReset))
        ;[0.15 0.15 0.15 0.5] Ai Locates and moves to player location
        (AI|Navigation|MovetoActor (AI|GetAIController self) Actor (Variables|Detection|GetTarget_Moveto_Radius) true true true 0))
      (else
        ;[0.15 0.15 0.15 0.5] DOes not see player so AI moves to Valid Location
        (AI|Navigation|MovetoLocation (AI|GetAIController self) Location -1.0 true true false true 0)))))

(fn FonDamageReceived
  (|CallParentFunction)
  (if (not (== (Variables|Default|GetLast_Attacker) self))
    (bind _player (Class|InterfaceCharatcerMaster|InterfaceCharacterType(Message) (Variables|Default|GetLast_Attacker)))
    (if _player
      (Movement|FAggroPlayer (Variables|Default|GetLast_Attacker)))))

(fn FAISetAnimationStance
  ;[0.15 0.15 0.15 0.5] Set animation
  (Class|BPIMixemoCharacter|InterfaceAnimationChange(Message) (Components|SkeletalMesh|GetAnimInstance (Variables|Character|GetMesh)) (Variables|Default|GetAnim%20Stance)))

(fn FAIAttack
  (bind _target (Variables|Default|GetTarget))
  (Utilities|IsValid _target
    (:Is%20Valid
      (Transformation|SetActorRotation (Math|Rotator|FindLookatRotation (Transformation|GetActorLocation) (Transformation|GetActorLocation _target))))))