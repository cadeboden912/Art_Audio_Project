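; Player controller that toggles a UI cursor mode on G, anchors the audio listener to the player pawn, swaps music and handles respawning.
; A music interface event fades out the current track and fades in the new one only when it differs.
; Respawn finds the nearest Actor_Respawn, then either spawns and possesses a fresh pawn, destroying the old one after a delay, or moves the existing pawn there.
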(event EventBeginPlay
  ;[0.15 0.15 0.15 0.5] Audio Plays at Player Location
  (Class|PlayerController|SetAudioListenerOverride (Variables|/Script/Engine.Actor|GetRootComponent (Game|Player|GetPlayerPawn 0)) "0, 0, 0" "0, 0, 0"))

(event EventMusicChangeInterface
  (params (Music :type Sound%20Cue%20Object%20Reference))
  (bind _fade_out_duration (Variables|Default|GetFade%20Out%20Duration))
  ;[0.15 0.15 0.15 0.5] Changes MUsic depneding on area
  (Variables|Default|SetMusic_New Music)
  (if (not (== (Variables|Default|GetMusic_New) (Variables|Default|GetMusic_Current)))
    (Audio|Components|Audio|FadeOut (Variables|Default|GetAudio) _fade_out_duration 0.0 "Linear" :!class /Script/Engine.AudioComponent)
    (Utilities|FlowControl|Delay _fade_out_duration)
    (Audio|Components|Audio|SetSound (Variables|Default|GetAudio) (Variables|Default|GetMusic_New))
    (Variables|Default|SetMusic_Current (Variables|Default|GetMusic_New))
    (Audio|Components|Audio|FadeIn (Variables|Default|GetAudio) 1.0 1.0 0.0 "Linear" :!class /Script/Engine.AudioComponent)))

(event EventInterfaceRespawn
  (params (New :type Boolean))
  (bind _returnvalue (Pawn|GetControlledPawn))
  (if New
    (Variables|Default|SetPawn_old _returnvalue)
    (Variables|Default|SetClass_Current (Utilities|GetClass _returnvalue))
    (bind _spawnlocation (CallFunction|FGetSpawnLocation))
    (Pawn|UnPossess)
    (bind _returnvalue_2 (Game|SpawnActorfromClass (Variables|Default|GetClass_Current) _spawnlocation "AlwaysSpawn" "MultiplyWithRoot" _returnvalue 0))
    (Pawn|Possess _returnvalue_2)
    (Utilities|FlowControl|Delay 3.0)
    (Actor|DestroyActor (Variables|Default|GetPawn_old))
    (Class|AbilityActivateInterface|InterfaceEventBeginPlay(Message) (Pawn|GetControlledPawn))
    (Class|InterfaceCharatcerMaster|InterfaceDeathState(Message) (Pawn|GetControlledPawn) false)
    (else
      (bind _spawnlocation_2 (CallFunction|FGetSpawnLocation))
      (Transformation|SetActorLocation (Pawn|GetControlledPawn) (.location _spawnlocation_2) false false)
      (Class|InterfaceCharatcerMaster|InterfaceDeathState(Message) (Pawn|GetControlledPawn) false))))

(event Input|KeyboardEvents|G
  (params (Key :type Key%20Structure :default "None"))
  ;[0.15 0.15 0.15 0.5] UI Interact activate
  (:Pressed
    (Utilities|FlowControl|FlipFlop
      (:A
        (Input|SetInputModeGameandUI self 0 "DoNotLock" true false)
        (Variables|Default|SetbShowMouseCursor true))
      (:B
        (Input|SetInputModeGameOnly self false)
        (Variables|Default|SetbShowMouseCursor false)))))

(fn ConstructionScript)

(fn FGetSpawnLocation
  (bind _outactors (Actor|GetAllActorsOfClass "/Game/Coursera/Actors/Respawn/Actor_Respawn.Actor_Respawn_C"))
  (bind _output_get (Variables|Default|SetLRespawn_Actors _outactors))
  (for _array_element _output_get
    (Utilities|Array|Add (Variables|Default|GetLRespawn_Distances) (Math|Vector|Distance(Vector) (Transformation|GetActorLocation _array_element) (Transformation|GetActorLocation (Pawn|GetControlledPawn)))))
  (return (Transformation|GetActorTransform (Utilities|Array|Get(acopy) (Variables|Default|GetLRespawn_Actors) (.IndexOfMinValue (Math|Float|MinOfFloatArray (Variables|Default|GetLRespawn_Distances)))))))